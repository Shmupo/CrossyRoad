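; BP_Log is a moving log that reacts when the chicken player touches it.
; On BeginPlay it picks its static mesh at random from the first two entries of LogList.
; Each Tick slides the Log component along its local Y axis at MaxSpeed, scaled by delta time.
; Overlap with BP_Chicky_Player only plays a loud 2D wood creak; the log applies nothing to the player.
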(event OnComponentBeginOverlap(Log)
  (params (OverlappedComponent :type Primitive%20Component%20Object%20Reference) (OtherActor :type Actor%20Object%20Reference) (OtherComp :type Primitive%20Component%20Object%20Reference) (OtherBodyIndex :type Integer) (bFromSweep :type Boolean) (SweepResult :type Hit%20Result%20Structure%20%28by%20ref%29))
  (bind _asbp_chicky_player (Utilities|Casting|CastToBP_Chicky_Player OtherActor))
  (Audio|PlaySound2D "/Game/StarterContent/Audio/Wood-creak.Wood-creak" 1e+01 1.0 0.0 0 0))

(event EventBeginPlay
  (CallFunction|SetLogMesh))

(event EventTick
  (params (DeltaSeconds :type Float%20%28single-precision%29))
  (Transformation|AddLocalOffset (Variables|Default|GetLog) (Math|Vector|MakeVector 0.0 (* DeltaSeconds (Variables|Default|GetMaxSpeed)) 0.0) false false))

(fn ConstructionScript)

(fn SetLogMesh
  (Components|StaticMesh|SetStaticMesh (Variables|Default|GetLog) (Utilities|Array|Get(acopy) (Variables|Default|GetLogList) (Math|Random|RandomInteger 2))))
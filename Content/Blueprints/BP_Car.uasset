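; BP_Car is a car hazard for the chicken player that slides along its local Y axis at MaxSpeed while Move is set.
; On overlap, RedCar disables the chicken's movement, squashes its mesh and plays a collapse sound at the world origin.
; FrontBox (stop for chicken or car) and LaneBox (one-time speed-up for chicken in lane) are both switched off by hardcoded false branches.
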(event OnComponentBeginOverlap(LaneBox)
  (params (OverlappedComponent :type Primitive%20Component%20Object%20Reference) (OtherActor :type Actor%20Object%20Reference) (OtherComp :type Primitive%20Component%20Object%20Reference) (OtherBodyIndex :type Integer) (bFromSweep :type Boolean) (SweepResult :type Hit%20Result%20Structure%20%28by%20ref%29))
  (Utilities|Casting|CastToBP_Chicky_Player OtherActor)
  ;[1 1 1] Turn on to make car speed up if chicken in lane
  (if false
    (Utilities|FlowControl|DoOnce false
      (:Completed
        (Variables|Default|SetMaxSpeed (* (Variables|Default|GetMaxSpeed) 1.5))))))

(event OnComponentBeginOverlap(RedCar)
  (params (OverlappedComponent :type Primitive%20Component%20Object%20Reference) (OtherActor :type Actor%20Object%20Reference) (OtherComp :type Primitive%20Component%20Object%20Reference) (OtherBodyIndex :type Integer) (bFromSweep :type Boolean) (SweepResult :type Hit%20Result%20Structure%20%28by%20ref%29))
  (bind _asbp_chicky_player (Utilities|Casting|CastToBP_Chicky_Player OtherActor))
  (Variables|/Game/Blueprints/BP_Chicky_Player.BP_Chicky_Player_C|SetCan_Move _asbp_chicky_player false)
  (Class|SceneComponent|AddLocalTransform (Variables|/Game/Blueprints/BP_Chicky_Player.BP_Chicky_Player_C|GetChicken _asbp_chicky_player) (Math|Transform|MakeTransform "0, 0, 0" "0, 0, 0" "1.000000,1.000000,0.100000") false false)
  (Audio|PlaySoundatLocation "/Game/StarterContent/Audio/Collapse01.Collapse01" "0, 0, 0" "0, 0, 0" 1.0 1.0 0.0 0 0 0 0))

(event OnComponentBeginOverlap(FrontBox)
  (params (OverlappedComponent :type Primitive%20Component%20Object%20Reference) (OtherActor :type Actor%20Object%20Reference) (OtherComp :type Primitive%20Component%20Object%20Reference) (OtherBodyIndex :type Integer) (bFromSweep :type Boolean) (SweepResult :type Hit%20Result%20Structure%20%28by%20ref%29))
  (Utilities|Casting|CastToBP_Chicky_Player OtherActor
    (:then
      _)
    (:CastFailed
      (Utilities|Casting|CastToBP_Car OtherActor)))
  ;[1 1 1] Turn on to make cars stop before hitting chicken
  (if false
    (Variables|Default|SetMove false)))

(event EventTick
  (params (DeltaSeconds :type Float%20%28single-precision%29))
  (if (Variables|Default|GetMove)
    (Transformation|AddLocalOffset (Variables|Default|GetRedCar) (Math|Vector|MakeVector 0.0 (* DeltaSeconds (Variables|Default|GetMaxSpeed)) 0.0) false false)))

(fn ConstructionScript)
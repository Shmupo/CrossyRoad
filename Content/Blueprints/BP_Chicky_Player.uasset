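; Player chicken character that moves in hops, counts steps and collects BP_Coin pickups with a sound and printed total.
; Axis input launches it up and along X or Y, gated by a half-second cooldown, while timelines turn the mesh toward the hop.
; Tick scrolls the camera along X, briefly reversing it after forward hops when its tracked DistanceBehindChicken exceeds a threshold.
; Left, Up and Right keys toggle walking audio.
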(event OnComponentBeginOverlap(Chicken)
  (params (OverlappedComponent :type Primitive%20Component%20Object%20Reference) (OtherActor :type Actor%20Object%20Reference) (OtherComp :type Primitive%20Component%20Object%20Reference) (OtherBodyIndex :type Integer) (bFromSweep :type Boolean) (SweepResult :type Hit%20Result%20Structure%20%28by%20ref%29))
  (bind _asbp_coin (Utilities|Casting|CastToBP_Coin OtherActor))
  (Actor|DestroyActor _asbp_coin)
  (bind _result (Math|Integer|IncrementInt (Variables|Default|GetCoinCounter))
    (:%20%20
      (Development|PrintString (Utilities|String|ToString(Integer) _result))
      (Audio|PlaySound2D "/Game/StarterContent/Audio/coin-pickup_Cue.coin-pickup_Cue" 1.0 1.0 0.0 0 0 false))))

(event Custom|MovementCooldown
  (Utilities|FlowControl|DoOnce false :!label _label
    (:Completed
      (Variables|Default|SetCan_Move false)
      (Utilities|FlowControl|Delay 0.5)
      (Variables|Default|SetCan_Move true)
      (goto _label Reset))))

(event EventTick
  (params (DeltaSeconds :type Float%20%28single-precision%29))
  (bind _cameraspeed (Variables|Default|GetCameraSpeed))
  ;[1 1 1] Camera
  (Transformation|AddWorldOffset (Variables|Default|GetCamera) (Math|Vector|MakeVector (select (and (Variables|Default|GetReverseCamera) (> (Variables|Default|GetDistanceBehindChicken) 1e+02)) (* DeltaSeconds (* _cameraspeed -1)) (* DeltaSeconds _cameraspeed)) 0.0 0.0) false false)
  (Variables|Default|SetDistanceBehindChicken (+ (select (and (Variables|Default|GetReverseCamera) (> (Variables|Default|GetDistanceBehindChicken) 1e+02)) (* DeltaSeconds (* _cameraspeed -1)) (* DeltaSeconds _cameraspeed)) (Variables|Default|GetDistanceBehindChicken)))
  (if (Variables|Default|GetCan_Move)
    (if (Variables|Default|GetReverseCamera)
      (Utilities|FlowControl|Delay 0.2)
      (Variables|Default|SetReverseCamera false))))

(event Input|AxisEvents|InputAxisMoveForward
  (params (AxisValue :type Float%20%28single-precision%29))
  (bind _chicken (Variables|Default|GetChicken))
  (bind _chicken_2 (Variables|Default|GetChicken))
  (if (and (> (Math|Float|Absolute(Float) AxisValue) 0.0) (Variables|Default|GetCan_Move))
    (CallFunction|MovementCooldown)
    (Variables|Default|SetStepCounter (+ (Variables|Default|GetStepCounter) 1))
    (Character|LaunchCharacter (Math|Vector|MakeVector (* AxisValue 2.4e+02) 0.0 1.9e+02) true true)
    (if (> AxisValue 0.3)
      (bind _newtrack_0 (Timeline|Timeline_0 PlayFromStart)
        (:Update
          (Transformation|SetWorldRotation _chicken (Math|Rotator|Lerp(Rotator) (Transformation|GetWorldRotation _chicken) "0,90.000000, 0" _newtrack_0 true) false false)
          (Variables|Default|SetReverseCamera true)))
      (else
        (bind _newtrack_0_2 (Timeline|Timeline_1 PlayFromStart)
          (:Update
            (Transformation|SetWorldRotation _chicken_2 (Math|Rotator|Lerp(Rotator) (Transformation|GetWorldRotation _chicken_2) "0,-90.000000, 0" _newtrack_0_2 true) false false)))))))

(event Input|AxisEvents|InputAxisMoveRight
  (params (AxisValue :type Float%20%28single-precision%29))
  (bind _chicken (Variables|Default|GetChicken))
  (bind _chicken_2 (Variables|Default|GetChicken))
  (if (and (Variables|Default|GetCan_Move) (> (Math|Float|Absolute(Float) AxisValue) 0.0))
    (CallFunction|MovementCooldown)
    (Variables|Default|SetStepCounter (+ (Variables|Default|GetStepCounter) 1))
    (Character|LaunchCharacter (Math|Vector|MakeVector 0.0 (* AxisValue 2.4e+02) 1.9e+02) true true)
    (if (> AxisValue 0.3)
      (bind _newtrack_0 (Timeline|Timeline_2 PlayFromStart)
        (:Update
          (Transformation|SetWorldRotation _chicken_2 (Math|Rotator|Lerp(Rotator) (Transformation|GetWorldRotation _chicken_2) "0,180.000000, 0" _newtrack_0 true) false false)))
      (else
        (bind _newtrack_0_2 (Timeline|Timeline_3 PlayFromStart)
          (:Update
            (Transformation|SetWorldRotation _chicken (Math|Rotator|Lerp(Rotator) (Transformation|GetWorldRotation _chicken) "0, 0, 0" _newtrack_0_2 true) false false)))))))

(event Input|KeyboardEvents|Up
  (params (Key :type Key%20Structure :default "None"))
  (bind _chicken_walking (Variables|Default|GetChicken%20walking))
  (:Pressed
    (Audio|Components|Audio|Play _chicken_walking 0.0))
  (:Released
    (Audio|Components|Audio|Stop _chicken_walking)))

(event Input|KeyboardEvents|Left
  (params (Key :type Key%20Structure :default "None"))
  (bind _chicken_walking (Variables|Default|GetChicken%20walking))
  (:Pressed
    (Audio|Components|Audio|Play _chicken_walking 0.0))
  (:Released
    (Audio|Components|Audio|Stop _chicken_walking)))

(event Input|KeyboardEvents|Right
  (params (Key :type Key%20Structure :default "None"))
  (bind _chicken_walking (Variables|Default|GetChicken%20walking))
  (:Pressed
    (Audio|Components|Audio|Play _chicken_walking 0.0))
  (:Released
    (Audio|Components|Audio|Stop _chicken_walking)))

(fn ConstructionScript)
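; BP_Lane is one lane in a Crossy Road-style game, with its type determined by its mesh's index in LaneList.
; LaneFullyMade spawns trees, rocks and coins, or timed logs, cars or trains from one side, plus a crossing on rail lanes.
; Edge triggers destroy arriving vehicles and logs and spawn replacements, delayed for trains.
; Player overlap with TriggerZone asks LaneSpawner for a new lane, then destroys this lane and its tracked actors.
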(event OnComponentBeginOverlap(TriggerZone)
  (params (OverlappedComponent :type Primitive%20Component%20Object%20Reference) (OtherActor :type Actor%20Object%20Reference) (OtherComp :type Primitive%20Component%20Object%20Reference) (OtherBodyIndex :type Integer) (bFromSweep :type Boolean) (SweepResult :type Hit%20Result%20Structure%20%28by%20ref%29))
  (Utilities|Casting|CastToBP_Chicky_Player OtherActor)
  (Default|SpawnLaneatSpawnPoint (Variables|Default|GetLaneSpawner))
  (Actor|DestroyActor)
  (for _array_element (Variables|Default|GetAllActorsMade)
    (Actor|DestroyActor _array_element)))

(event OnComponentBeginOverlap(CarTriggerZoneLeft)
  (params (OverlappedComponent :type Primitive%20Component%20Object%20Reference) (OtherActor :type Actor%20Object%20Reference) (OtherComp :type Primitive%20Component%20Object%20Reference) (OtherBodyIndex :type Integer) (bFromSweep :type Boolean) (SweepResult :type Hit%20Result%20Structure%20%28by%20ref%29))
  (bind _asbp_car (Utilities|Casting|CastToBP_Car OtherActor)
    (:then
      (Actor|DestroyActor _asbp_car)
      (CallFunction|SpawnEntities))
    (:CastFailed
      (bind _asbp_log (Utilities|Casting|CastToBP_Log OtherActor)
        (:then
          (Actor|DestroyActor _asbp_log)
          (CallFunction|SpawnEntities))
        (:CastFailed
          (bind _asbp_train (Utilities|Casting|CastToBP_Train OtherActor))
          (Actor|DestroyActor _asbp_train)
          (Utilities|FlowControl|Delay 4.0)
          (CallFunction|SpawnEntities))))))

(event OnComponentBeginOverlap(CarTriggerZoneRight)
  (params (OverlappedComponent :type Primitive%20Component%20Object%20Reference) (OtherActor :type Actor%20Object%20Reference) (OtherComp :type Primitive%20Component%20Object%20Reference) (OtherBodyIndex :type Integer) (bFromSweep :type Boolean) (SweepResult :type Hit%20Result%20Structure%20%28by%20ref%29))
  (bind _asbp_car (Utilities|Casting|CastToBP_Car OtherActor)
    (:then
      (Actor|DestroyActor _asbp_car)
      (CallFunction|SpawnEntities))
    (:CastFailed
      (bind _asbp_log (Utilities|Casting|CastToBP_Log OtherActor)
        (:then
          (Actor|DestroyActor _asbp_log)
          (CallFunction|SpawnEntities))
        (:CastFailed
          (bind _asbp_train (Utilities|Casting|CastToBP_Train OtherActor))
          (Actor|DestroyActor _asbp_train)
          (Utilities|FlowControl|Delay 4.0)
          (CallFunction|SpawnEntities))))))

(event Custom|TrySpawn
  ;[1 1 1] SpawnTiming
  (Utilities|FlowControl|Delay (Math|Random|RandomFloatinRange 2.0 5.0))
  (CallFunction|SpawnEntities))

(event Custom|LaneFullyMade
  ;[1 1 1] SpawnTiming
  (if (== (Utilities|Array|FindItem (Variables|Default|GetLaneList) (Variables|/Script/Engine.StaticMeshComponent|GetStaticMesh (Variables|Components|GetLaneMesh))) 0)
    (CallFunction|TreeRockSpawn)
    (elif (== (Utilities|Array|FindItem (Variables|Default|GetLaneList) (Variables|/Script/Engine.StaticMeshComponent|GetStaticMesh (Variables|Components|GetLaneMesh))) 4)
      (CallFunction|RRCrossingSpawn)
      (Utilities|Time|SetTimerbyEvent (delegate Custom|TrySpawn) 0.0)
      (Utilities|FlowControl|Delay (Math|Random|RandomFloatinRange 2.0 5.0))
      (CallFunction|SpawnEntities)
      (else
        (Utilities|Time|SetTimerbyEvent (delegate Custom|TrySpawn) 0.5 true)))))

(fn ConstructionScript)

(fn SetLaneMesh
  (params (Lane%20No. :type Integer))
  (bind _returnvalue (Components|StaticMesh|SetStaticMesh (Variables|Components|GetLaneMesh) (Utilities|Array|Get(acopy) (Variables|Default|GetLaneList) Lane%20No.)))
  (switch int (Math|Conversions|ToInteger(Boolean) _returnvalue)
    (:0
      _)
    (:1
      (Variables|Default|SetRightSpawn (Math|Random|RandomBool) :!label _label))
    (:2
      (goto _label))
    (:3
      (goto _label)))
  (return 0))

(fn SpawnEntities
  (switch int (Utilities|Array|FindItem (Variables|Default|GetLaneList) (Variables|/Script/Engine.StaticMeshComponent|GetStaticMesh (Variables|Components|GetLaneMesh)))
    (:1
      (CallFunction|LogSpawn))
    (:2
      (CallFunction|CarSpawn :!label _label))
    (:3
      (goto _label))
    (:4
      (CallFunction|TrainSpawn))))

(fn TreeRockSpawn
  (bind _allactorsmade (Variables|Default|GetAllActorsMade))
  (bind _treespawnpos (Variables|Default|GetTreeSpawnPos))
  (bind _returnvalue (Transformation|GetSocketLocation _treespawnpos "None"))
  (bind _returnvalue_2 (Game|SpawnActorfromClass "/Game/Blueprints/BP_Tree.BP_Tree_C" (Math|Transform|MakeTransform (Transformation|GetWorldLocation (Variables|Components|GetEntitySpawnRight)) "0, 0, 0" "1.000000,1.000000,1.000000") "Undefined" 0 0))
  (bind _returnvalue_3 (Game|SpawnActorfromClass "/Game/Blueprints/BP_Tree.BP_Tree_C" (Math|Transform|MakeTransform (Transformation|GetWorldLocation (Variables|Components|GetEntitySpawnLeft)) "0, 0, 0" "1.000000,1.000000,1.000000") "Undefined" 0 0))
  (Utilities|Array|Add _allactorsmade _returnvalue_2)
  (Utilities|Array|Add _allactorsmade _returnvalue_3)
  ;[1 1 1] Spawning Random Trees/Rocks
  (for _index (range 1 10)
    (if (>= 0.3 (Math|Random|RandomFloat))
      (bind _asactor (Utilities|Casting|CastToActorClass (Class|KismetMathLibrary|SelectClass (Class|KismetMathLibrary|SelectClass "/Game/Blueprints/BP_Tree.BP_Tree_C" "/Game/Blueprints/BP_Rock.BP_Rock_C" (Math|Random|RandomBool)) "/Game/Blueprints/BP_Coin.BP_Coin_C" (Math|Random|RandomBool))))
      (Game|SpawnActorfromClass _asactor (Math|Transform|MakeTransform (Math|Vector|MakeVector (.x _returnvalue) (+ (* _index 80) (.y _returnvalue)) (.z _returnvalue)) "0,4.000000, 0" "1.000000,1.000000,1.000000") "Undefined" 0 0))))

(fn CarSpawn
  (bind _entityspawnleft (Variables|Components|GetEntitySpawnLeft))
  (bind _rightspawn (Variables|Default|GetRightSpawn))
  (bind _entityspawnright (Variables|Components|GetEntitySpawnRight))
  (bind _returnvalue (Transformation|GetWorldLocation _entityspawnleft))
  (bind _returnvalue_2 (Transformation|GetWorldLocation _entityspawnright))
  (bind _returnvalue_3 (select _rightspawn _returnvalue_2 _returnvalue))
  (if _rightspawn
    (bind _returnvalue_4 (Game|SpawnActorfromClass "/Game/Blueprints/BP_Car.BP_Car_C" (Math|Transform|MakeTransform _returnvalue_3 "0,-90.000000, 0" "1.000000,1.000000,1.000000") "Undefined" 0 0))
    (Utilities|Array|Add (Variables|Default|GetAllActorsMade) _returnvalue_4)
    (else
      (bind _returnvalue_5 (Game|SpawnActorfromClass "/Game/Blueprints/BP_Car.BP_Car_C" (Math|Transform|MakeTransform _returnvalue_3 "0,90.000000, 0" "1.000000,1.000000,1.000000") "Undefined" 0 0))
      (Utilities|Array|Add (Variables|Default|GetAllActorsMade) _returnvalue_5))))

(fn LogSpawn
  (bind _entityspawnleft (Variables|Components|GetEntitySpawnLeft))
  (bind _rightspawn (Variables|Default|GetRightSpawn))
  (bind _entityspawnright (Variables|Components|GetEntitySpawnRight))
  (bind _returnvalue (Transformation|GetWorldLocation _entityspawnleft))
  (bind _returnvalue_2 (Transformation|GetWorldLocation _entityspawnright))
  (bind _returnvalue_3 (select _rightspawn _returnvalue_2 _returnvalue))
  (if _rightspawn
    (bind _returnvalue_4 (Game|SpawnActorfromClass "/Game/Blueprints/BP_Log.BP_Log_C" (Math|Transform|MakeTransform _returnvalue_3 "0,-90.000000, 0" "1.000000,1.000000,1.000000") "Undefined" 0 0))
    (Utilities|Array|Add (Variables|Default|GetAllActorsMade) _returnvalue_4)
    (else
      (bind _returnvalue_5 (Game|SpawnActorfromClass "/Game/Blueprints/BP_Log.BP_Log_C" (Math|Transform|MakeTransform _returnvalue_3 "0,90.000000, 0" "1.000000,1.000000,1.000000") "Undefined" 0 0))
      (Utilities|Array|Add (Variables|Default|GetAllActorsMade) _returnvalue_5))))

(fn TrainSpawn
  (bind _entityspawnleft (Variables|Components|GetEntitySpawnLeft))
  (bind _rightspawn (Variables|Default|GetRightSpawn))
  (bind _entityspawnright (Variables|Components|GetEntitySpawnRight))
  (bind _returnvalue (Transformation|GetWorldLocation _entityspawnleft))
  (bind _returnvalue_2 (Transformation|GetWorldLocation _entityspawnright))
  (bind _returnvalue_3 (select _rightspawn _returnvalue_2 _returnvalue))
  (if _rightspawn
    (bind _returnvalue_4 (Game|SpawnActorfromClass "/Game/Blueprints/BP_Train.BP_Train_C" (Math|Transform|MakeTransform _returnvalue_3 "0,-90.000000, 0" "1.000000,1.000000,1.000000") "Undefined" 0 0))
    (Utilities|Array|Add (Variables|Default|GetAllActorsMade) _returnvalue_4)
    (else
      (bind _returnvalue_5 (Game|SpawnActorfromClass "/Game/Blueprints/BP_Train.BP_Train_C" (Math|Transform|MakeTransform _returnvalue_3 "0,90.000000, 0" "1.000000,1.000000,1.000000") "Undefined" 0 0))
      (Utilities|Array|Add (Variables|Default|GetAllActorsMade) _returnvalue_5))))

(fn RRCrossingSpawn
  (bind _rr_crossing_pos (Variables|Default|GetRR_Crossing_Pos))
  (bind _returnvalue (Transformation|GetWorldLocation _rr_crossing_pos))
  (if true
    (Game|SpawnActorfromClass "/Game/Blueprints/BP_RR-Crossing.BP_RR-Crossing_C" (Math|Transform|MakeTransform (Math|Vector|MakeVector (.x _returnvalue) (.y _returnvalue) (.z _returnvalue)) "0, 0, 0" "1.000000,1.000000,1.000000") "Undefined" 0 0)))
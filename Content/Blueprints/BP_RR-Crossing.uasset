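; BP_RR-Crossing is an actor, named as a railroad crossing, that flashes a blue and a red point light in alternation.
; Tick counts down by delta time and, every half second, resets the countdown and flips a boolean.
; That boolean selects which light gets full intensity while the other drops to zero.
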(event EventBeginPlay)

(event Collision|EventActorBeginOverlap
  (params (OtherActor :type Actor%20Object%20Reference)))

(event EventTick
  (params (DeltaSeconds :type Float%20%28single-precision%29))
  (bind _pointlight_blue (Variables|Default|GetPointLight_Blue))
  (bind _pointlight_red (Variables|Default|GetPointLight_Red))
  (bind _output_get (Variables|Default|SetCountdown (- (Variables|Default|GetCountdown) DeltaSeconds)))
  (if (<= _output_get 0.0)
    (Variables|Default|SetCountdown 0.5)
    (bind _output_get_2 (Variables|Default|SetLightType (not (Variables|Default|GetLightType))))
    (if _output_get_2
      (Rendering|Components|Light|SetIntensity _pointlight_blue 1e+04)
      (Rendering|Components|Light|SetIntensity _pointlight_red 0.0)
      (else
        (Rendering|Components|Light|SetIntensity _pointlight_blue 0.0)
        (Rendering|Components|Light|SetIntensity _pointlight_red 1e+04)))))

(fn ConstructionScript)
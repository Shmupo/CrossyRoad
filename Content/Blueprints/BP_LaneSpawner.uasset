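; BP_LaneSpawner builds a chain of BP_Lane actors of random terrain (grass, railroad, road, water per comments), apparently for a lane-crossing game.
; On BeginPlay it lays an initial batch from just behind the player, each at the previous lane's SpawnPoint, passing itself to each.
; After the first few lanes, ConsecutiveSpawn picks types in random-length runs, remapping some indices within runs, to set each lane's mesh.
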(event EventBeginPlay
  (CallFunction|SpawnInitialLanes))

(event Collision|EventActorBeginOverlap
  (params (OtherActor :type Actor%20Object%20Reference)))

(event EventTick
  (params (DeltaSeconds :type Float%20%28single-precision%29)))

(fn ConstructionScript)

(fn SpawnLane
  (params (SpawnLocation :type Vector))
  (bind _returnvalue (Game|SpawnActorfromClass "/Game/Blueprints/BP_Lane.BP_Lane_C" (Math|Transform|MakeTransform SpawnLocation "0, 0, 0" "1.000000,1.000000,1.000000") "Undefined" 0 0))
  (bind _output_get (Variables|Default|SetNewestLane _returnvalue))
  (Variables|/Game/Blueprints/BP_Lane.BP_Lane_C|SetLaneSpawner _output_get self))

(fn SpawnLaneatSpawnPoint
  (bind _newestlane (Variables|Default|GetNewestLane))
  (bind _result (Math|Integer|IncrementInt (Variables|Default|GetLanesMade))
    (:%20%20
      (CallFunction|SpawnLane (Transformation|GetWorldLocation (Variables|/Game/Blueprints/BP_Lane.BP_Lane_C|GetSpawnPoint (Variables|Default|GetNewestLane))))
      (if (> _result 5)
        (bind _lane_no_ (CallFunction|ConsecutiveSpawn))
        (Default|SetLaneMesh _newestlane _lane_no_)
        (Default|LaneFullyMade _newestlane)))))

(fn SpawnInitialLanes
  (for _index (range 0 20)
    (Utilities|IsValid (Variables|Default|GetNewestLane)
      (:Is%20Valid
        (CallFunction|SpawnLaneatSpawnPoint))
      (:Is%20Not%20Valid
        (CallFunction|SpawnLane (+ (Transformation|GetActorLocation (Game|Player|GetPlayerPawn 0)) "-240.000000,0,0"))))))

(fn ConsecutiveSpawn
  (bind _returnvalue (Math|Random|RandomIntegerinRange 0 3))
  (if (< (Variables|Default|GetLaneTypeSpawned) (Variables|Default|GetLaneTypeToSpawn))
    (if (== (Variables|Default|GetLaneChosen) 3)
      (Variables|Default|SetLaneChosen 2))
    (Math|Integer|IncrementInt (Variables|Default|GetLaneTypeSpawned) :!label _label
      (:%20%20
        (return (Variables|Default|GetLaneChosen))))
    (else
      (Variables|Default|SetLaneTypeToSpawn (Utilities|Select :Index _returnvalue :Option%200 (Math|Random|RandomIntegerinRange 1 2) :Option%201 (Math|Random|RandomIntegerinRange 1 5) :Option%202 (Math|Random|RandomIntegerinRange 1 10) :Option%203 (Math|Random|RandomIntegerinRange 1 2)))
      (Variables|Default|SetLaneTypeSpawned 0)
      (bind _output_get (Variables|Default|SetLaneChosen (select (== _returnvalue (Variables|Default|GetLaneChosen)) 0 _returnvalue)))
      (if (== _output_get 3)
        (Variables|Default|SetLaneChosen 4)
        (goto _label)
        (elif (== _output_get 2)
          (Variables|Default|SetLaneChosen 3)
          (goto _label))))))